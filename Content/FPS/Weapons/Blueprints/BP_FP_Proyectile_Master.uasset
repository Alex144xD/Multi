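; Master projectile Blueprint for first-person weapons, with server-authoritative direct-hit or explosive behavior selected by IsExplosive.
; Non-explosive rounds pass server hits to a client-named event that applies damage and destroys them after a short delay; mesh hits also destroy them.
; Explosive rounds destroy themselves when movement stops, then apply radial damage on the server and call multicast explosion sound and particles.
; The impact FX event is empty, leaving its effect nodes disconnected.
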(event OnComponentHit(SM_Proyectile)
  (params (HitComponent :type Primitive%20Component%20Object%20Reference) (OtherActor :type Actor%20Object%20Reference) (OtherComp :type Primitive%20Component%20Object%20Reference) (NormalImpulse :type Vector :default "0, 0, 0") (Hit :type Hit%20Result%20Structure%20%28by%20ref%29))
  (if (not (Variables|Default|GetisExplosive?))
    (Utilities|FlowControl|Delay 0.2)
    (Actor|DestroyActor)))

(event OnProjectileStop(ProjectileMovement)
  (params (ImpactResult :type Hit%20Result%20Structure%20%28by%20ref%29))
  (Networking|SwitchHasAuthority
    (:Authority
      (if (Variables|Default|GetisExplosive?)
        (Actor|DestroyActor)))))

(event Custom|Client_OnHit
  (params (HitResult :type Hit%20Result%20Structure))
  (if (not (Variables|Default|GetisExplosive?))
    (Game|Damage|ApplyDamage (.HitActor (Collision|BreakHitResult HitResult)) (Math|Conversions|ToFloat(Integer) (Variables|Default|GetDamage)) (Game|GetInstigatorController) self)
    (CallFunction|ClientProjectileFx HitResult)
    (Utilities|FlowControl|Delay 0.2)
    (Actor|DestroyActor)))

(event Custom|ClientProjectileFx
  (params (HitResult :type Hit%20Result%20Structure)))

(event Custom|MulticastExplosionFX
  (bind _returnvalue (Transformation|GetActorLocation))
  (Audio|PlaySoundatLocation (Variables|Default|GetExplosionCue) _returnvalue)
  (Effects|SpawnEmitteratLocation (Variables|Default|GetExplosionPS) _returnvalue (Transformation|GetActorRotation)))

(event EventDestroyed
  (Networking|SwitchHasAuthority
    (:Authority
      (if (Variables|Default|GetisExplosive?)
        (Game|Damage|ApplyRadialDamage (Math|Conversions|ToFloat(Integer) (Variables|Default|GetDamage)) (Transformation|GetActorLocation) (Variables|Default|GetdamageRadius) 0 0 self (Game|GetInstigatorController) false "ECC_Visibility")
        (CallFunction|MulticastExplosionFX)))))

(event Collision|EventHit
  (params (MyComp :type Primitive%20Component%20Object%20Reference) (Other :type Actor%20Object%20Reference) (OtherComp :type Primitive%20Component%20Object%20Reference) (bSelfMoved :type Boolean) (HitLocation :type Vector :default "0, 0, 0") (HitNormal :type Vector :default "0, 0, 0") (NormalImpulse :type Vector :default "0, 0, 0") (Hit :type Hit%20Result%20Structure%20%28by%20ref%29))
  (Networking|SwitchHasAuthority
    (:Authority
      (if (not (Variables|Default|GetisExplosive?))
        (CallFunction|ClientonHit Hit)))))

(event EventBeginPlay
  (Utilities|FlowControl|Sequence
    (:then_0
      (Networking|SwitchHasAuthority
        (:Authority
          (Collision|IgnoreActorwhenMoving (Variables|Default|GetProyectile_Collision) (Game|GetInstigator) true))))))

(fn ConstructionScript)

(fn OnRepDamageRadius)