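; Base replicated projectile for FPS weapons, switching between bullet-style and explosive behavior through IsExplosive.
; The server ignores the instigator for collision and, on a non-explosive hit, applies point-of-contact damage, multicasts impact effects and destroys the actor after a short delay.
; When explosive projectile movement stops, the server multicasts explosion sound and particles with immediate destruction.
; The radial damage logic is disconnected, so explosions deal no damage here.
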(event OnProjectileStop(ProjectileMovement)
  (params (ImpactResult :type Hit%20Result%20Structure%20%28by%20ref%29))
  (Networking|SwitchHasAuthority
    (:Authority
      (if (Variables|Default|GetisExplosive?)
        (CallFunction|MulticastExplosionFX)))))

(event OnComponentHit(TP_StaticMesh)
  (params (HitComponent :type Primitive%20Component%20Object%20Reference) (OtherActor :type Actor%20Object%20Reference) (OtherComp :type Primitive%20Component%20Object%20Reference) (NormalImpulse :type Vector :default "0, 0, 0") (Hit :type Hit%20Result%20Structure%20%28by%20ref%29)))

(event Custom|Server_OnHit
  (params (HitResult :type Hit%20Result%20Structure))
  (if (not (Variables|Default|GetisExplosive?))
    (Game|Damage|ApplyDamage (.HitActor (Collision|BreakHitResult HitResult)) (Math|Conversions|ToFloat(Integer) (Variables|Default|GetDamage)) (Game|GetInstigatorController) self)
    (CallFunction|MulticastProjectileFx HitResult)
    (Utilities|FlowControl|Delay 0.2)
    (Actor|DestroyActor)))

(event Custom|MulticastProjectileFx
  (params (HitResult :type Hit%20Result%20Structure))
  (bind (_bblockinghit _binitialoverlap _time _location _impactpoint _normal _impactnormal _physmat _hitactor _hitcomponent _hitbonename _hititem _faceindex _tracestart) (Collision|BreakHitResult HitResult))
  (Audio|PlaySoundatLocation (Variables|Default|GetImpactSound) _tracestart)
  (Effects|SpawnEmitteratLocation (Variables|Default|GetImpactEffect) _impactpoint (Math|Rotator|MakeRotfromZ _impactnormal)))

(event Custom|MulticastExplosionFX
  (bind _returnvalue (Transformation|GetActorLocation))
  (Audio|PlaySoundatLocation (Variables|Default|GetExplosionCue) _returnvalue)
  (Effects|SpawnEmitteratLocation (Variables|Default|GetExplosionPS) _returnvalue (Transformation|GetActorRotation))
  (Actor|DestroyActor))

(event EventDestroyed)

(event Collision|EventHit
  (params (MyComp :type Primitive%20Component%20Object%20Reference) (Other :type Actor%20Object%20Reference) (OtherComp :type Primitive%20Component%20Object%20Reference) (bSelfMoved :type Boolean) (HitLocation :type Vector :default "0, 0, 0") (HitNormal :type Vector :default "0, 0, 0") (NormalImpulse :type Vector :default "0, 0, 0") (Hit :type Hit%20Result%20Structure%20%28by%20ref%29))
  (Networking|SwitchHasAuthority
    (:Authority
      (if (not (Variables|Default|GetisExplosive?))
        (CallFunction|ServeronHit Hit)))))

(event EventBeginPlay
  (Utilities|FlowControl|Sequence
    (:then_0
      (Networking|SwitchHasAuthority
        (:Authority
          (Collision|IgnoreActorwhenMoving (Variables|Default|GetProyectile_Collision) (Game|GetInstigator) true))))))

(fn ConstructionScript)