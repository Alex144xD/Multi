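; Master weapon Blueprint for a multiplayer FPS, handling single, auto and multi-round fire plus timeline-driven scope zoom.
; Client fire sphere-traces from the camera with spread, then from the muzzle toward that point, and sends the result to the server.
; The server applies hitscan damage or spawns separate first- and third-person projectiles, then multicasts effects.
; Muzzle flashes are owner-filtered per mesh; auto fire loops through a gate, and multifire plays one flash per trigger pull.
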(event Custom|ClientActivateScope
  (bind _bpcharactermasterref (Variables|Default|GetBPCharacterMasterRef))
  ;[1 1 1] Activate/Deactivate Scope
  (bind (_direction _zoomamount _scopeopacity) (Timeline|ScopeTimeline Play)
    (:Update
      (Camera|SetFieldOfView (Variables|/Game/FPS/Characters/Blueprints/BP_Character_Master.BP_Character_Master_C|GetFPCam _bpcharactermasterref) _zoomamount)
      (bind _aspc_mp_fps (Utilities|Casting|CastToPC_MP_FPS (Pawn|GetController _bpcharactermasterref)))
      (bind _ashud_mp_fps (Utilities|Casting|CastToHUD_MP_FPS (HUD|GetHUD _aspc_mp_fps)))
      (Variables|/Game/FPS/Characters/Blueprints/HUD_MP_FPS.HUD_MP_FPS_C|SetScopeOpacity _ashud_mp_fps _scopeopacity))))

(event Custom|ServerShootInfo
  (params (HitResult :type Hit%20Result%20Structure) (Hit :type Boolean) (FPProyectileSpawn :type Vector) (TPProyectileSpawn :type Vector))
  (bind (_bblockinghit _binitialoverlap _time _location _impactpoint _normal _impactnormal _physmat _hitactor _hitcomponent _hitbonename _hititem _faceindex _tracestart _traceend) (Collision|BreakHitResult HitResult))
  (bind (_bblockinghit_2 _binitialoverlap_2 _time_2 _location_2 _impactpoint_2 _normal_2 _impactnormal_2 _physmat_2 _hitactor_2 _hitcomponent_2 _hitbonename_2 _hititem_2 _faceindex_2 _tracestart_2 _traceend_2) (Collision|BreakHitResult HitResult))
  (if (Variables|Default|GetIsHitScan?)
    (Game|Damage|ApplyDamage (.HitActor (Collision|BreakHitResult HitResult)) (Math|Conversions|ToFloat(Integer) (Variables|Default|GetDamage)) (Game|GetInstigatorController) self)
    (else
      (Game|SpawnActorfromClass (Variables|Default|GetTPProjectile) (Math|Transform|MakeTransform TPProyectileSpawn (Math|Rotator|FindLookatRotation TPProyectileSpawn (Math|Vector|SelectVector _impactpoint _traceend Hit))) "AlwaysSpawn" (Components|GetOwner) (Game|GetInstigator))
      (Game|SpawnActorfromClass (Variables|Default|GetFPProjectile) (Math|Transform|MakeTransform FPProyectileSpawn (Math|Rotator|FindLookatRotation FPProyectileSpawn (Math|Vector|SelectVector _impactpoint_2 _traceend_2 Hit))) "AlwaysSpawn" 0 0)))
  (switch Utilities|FlowControl|Switch|SwitchonE_FiringModes (Variables|Default|GetFiringMode)
    (:NewEnumerator0
      (CallFunction|MulticastSingleFireWeaponFX HitResult Hit :!label _label))
    (:NewEnumerator1
      (goto _label))
    (:NewEnumerator2
      (CallFunction|MulticastMultiFireWeaponFX HitResult Hit))))

(event Custom|Client_ShootInfo
  (params (%20HitResult :type Hit%20Result%20Structure) (hit :type Boolean))
  (if (Variables|Default|GetIsHitScan?)
    _))

(event Custom|Client_OnWeaponFire
  (bind _bpcharactermasterref (Variables|Default|GetBPCharacterMasterRef))
  (bind _array (Utilities|Array|MakeArray _bpcharactermasterref))
  (bind _fpcam (Variables|/Game/FPS/Characters/Blueprints/BP_Character_Master.BP_Character_Master_C|GetFPCam _bpcharactermasterref))
  (bind _returnvalue (Transformation|GetWorldLocation _fpcam))
  (switch Utilities|FlowControl|Switch|SwitchonE_FiringModes (Variables|Default|GetFiringMode)
    (:NewEnumerator0
      _)
    (:NewEnumerator1
      (Utilities|Autofire
        (:then_0
          _)))
    (:NewEnumerator2
      (Utilities|Multifire
        (:LoopBody
          _))))
  (bind (_outhit _returnvalue_2) (Collision|SphereTraceByChannel _returnvalue (Utilities|AddRandomSpread (+ _returnvalue (* (Math|Vector|GetForwardVector (Transformation|GetWorldRotation _fpcam)) (Variables|Default|GetSphereTraceRange)))) (Variables|Default|GetSphereTraceRadious) "TraceTypeQuery1" false _array "None"))
  (bind (_outhit_2 _returnvalue_3) (Collision|SphereTraceByChannel (Transformation|GetSocketLocation (Variables|Default|GetSK_FP_Mesh) (Variables|Default|GetMuzzleSocketName)) (Math|Vector|SelectVector (.ImpactPoint (Collision|BreakHitResult _outhit)) (.TraceEnd (Collision|BreakHitResult _outhit)) _returnvalue_2) (Variables|Default|GetSphereTraceRadious) "TraceTypeQuery1" false _array "None"))
  (CallFunction|ServerShootInfo _outhit_2 _returnvalue_3 (Transformation|GetSocketLocation (Variables|Default|GetSK_FP_Mesh) (Variables|Default|GetMuzzleSocketName)) (Transformation|GetSocketLocation (Variables|Default|GetSK_TP_Weapon) (Variables|Default|GetMuzzleSocketName))))

(event Custom|Client_OffWeaponFire
  (bind _bpcharactermasterref (Variables|Default|GetBPCharacterMasterRef))
  (bind _array (Utilities|Array|MakeArray _bpcharactermasterref))
  (bind _fpcam (Variables|/Game/FPS/Characters/Blueprints/BP_Character_Master.BP_Character_Master_C|GetFPCam _bpcharactermasterref))
  (bind _returnvalue (Transformation|GetWorldLocation _fpcam))
  (Utilities|FlowControl|Sequence
    (:then_0
      (Utilities|Autofire) ; enters at Close
    )
    (:then_1
      (CallFunction|ServerOffWeaponFire))))

(event Custom|ServerOffWeaponFire
  (Utilities|FlowControl|Sequence
    (:then_0
      (Utilities|FlowControl|Delay (Variables|Default|GetWeaponCoolDown))
      (Variables|Default|SetIsCooldownActive? false))
    (:then_1
      (CallFunction|MulticastOffWeaponFire))))

(event Custom|MulticastSingleFireWeaponFX
  (params (HitResult :type Hit%20Result%20Structure) (Hit :type Boolean))
  (CallFunction|SingleFireFX HitResult Hit))

(event Custom|MulticastOffWeaponFire
  (Utilities|FlowControl|Sequence
    (:then_0
      (Utilities|MultifireDoOnceFX) ; enters at Reset
    )))

(event Custom|ClientDeActivateScope
  (bind _bpcharactermasterref (Variables|Default|GetBPCharacterMasterRef))
  ;[1 1 1] Activate/Deactivate Scope
  (bind (_direction _zoomamount _scopeopacity) (Timeline|ScopeTimeline Reverse)
    (:Update
      (Camera|SetFieldOfView (Variables|/Game/FPS/Characters/Blueprints/BP_Character_Master.BP_Character_Master_C|GetFPCam _bpcharactermasterref) _zoomamount)
      (bind _aspc_mp_fps (Utilities|Casting|CastToPC_MP_FPS (Pawn|GetController _bpcharactermasterref)))
      (bind _ashud_mp_fps (Utilities|Casting|CastToHUD_MP_FPS (HUD|GetHUD _aspc_mp_fps)))
      (Variables|/Game/FPS/Characters/Blueprints/HUD_MP_FPS.HUD_MP_FPS_C|SetScopeOpacity _ashud_mp_fps _scopeopacity))))

(event Custom|MulticastAutoFireWeapoFX
  (params (HitResult :type Hit%20Result%20Structure) (Hit :type Boolean))
  (Utilities|FlowControl|Sequence
    (:then_0
      (CallFunction|AutoFireFX HitResult Hit))))

(event Custom|MulticastMultiFireWeaponFX
  (params (HitResult :type Hit%20Result%20Structure) (Hit :type Boolean))
  (Utilities|FlowControl|Sequence
    (:then_0
      (CallFunction|MultiFireFX HitResult Hit))
    (:then_1
      (Utilities|MultifireDoOnceFX))))

(event EventBeginPlay)

(event Collision|EventActorBeginOverlap
  (params (OtherActor :type Actor%20Object%20Reference)))

(event EventTick
  (params (DeltaSeconds :type Float%20%28single-precision%29)))

(fn ConstructionScript)

(fn SingleFireFX
  (params (Hit :type Hit%20Result%20Structure%20%28by%20ref%29) (Condition :type Boolean))
  (bind (_bblockinghit _binitialoverlap _time _location _impactpoint _normal _impactnormal) (Collision|BreakHitResult Hit))
  (bind _sk_fp_mesh (Variables|Default|GetSK_FP_Mesh))
  (Audio|SpawnSoundAttached (Variables|Default|GetFireWeaponSound) _sk_fp_mesh "Muzzle")
  (Utilities|FlowControl|Sequence
    (:then_0
      (bind _returnvalue (Effects|SpawnEmitterAttached (Variables|Default|GetPSMuzzleFlash) _sk_fp_mesh (Variables|Default|GetMuzzleSocketName)))
      (Rendering|SetOnlyOwnerSee _returnvalue true :!class /Script/Engine.PrimitiveComponent)
      (if (Variables|Default|GetIsHitScan?)
        (if Condition
          (Audio|PlaySoundatLocation (Variables|Default|GetImpactSound) _location)
          (Effects|SpawnEmitteratLocation (Variables|Default|GetImpactEffect) _location (Math|Rotator|MakeRotfromZ _impactnormal)))))
    (:then_1
      (bind _returnvalue_2 (Effects|SpawnEmitterAttached (Variables|Default|GetPSMuzzleFlash) (Variables|Default|GetSK_TP_Weapon) (Variables|Default|GetMuzzleSocketName)))
      (Class|PrimitiveComponent|SetOwnerNoSee _returnvalue_2 true))))

(fn MultiFireFX
  (params (Hit :type Hit%20Result%20Structure%20%28by%20ref%29) (Condition :type Boolean))
  (bind (_bblockinghit _binitialoverlap _time _location _impactpoint _normal _impactnormal) (Collision|BreakHitResult Hit))
  (if (Variables|Default|GetIsHitScan?)
    (if Condition
      (Audio|PlaySoundatLocation (Variables|Default|GetImpactSound) _location)
      (Effects|SpawnEmitteratLocation (Variables|Default|GetImpactEffect) _location (Math|Rotator|MakeRotfromZ _impactnormal)))))

(fn AutoFireFX
  (params (Hit :type Hit%20Result%20Structure%20%28by%20ref%29) (Condition :type Boolean))
  (bind (_bblockinghit _binitialoverlap _time _location _impactpoint _normal _impactnormal) (Collision|BreakHitResult Hit))
  (bind _sk_fp_mesh (Variables|Default|GetSK_FP_Mesh))
  (Audio|SpawnSoundAttached (Variables|Default|GetFireWeaponSound) _sk_fp_mesh "Muzzle")
  (Utilities|FlowControl|Sequence
    (:then_0
      (bind _returnvalue (Effects|SpawnEmitterAttached (Variables|Default|GetPSMuzzleFlash) _sk_fp_mesh (Variables|Default|GetMuzzleSocketName)))
      (Rendering|SetOnlyOwnerSee _returnvalue true :!class /Script/Engine.PrimitiveComponent)
      (if (Variables|Default|GetIsHitScan?)
        (if Condition
          (Audio|PlaySoundatLocation (Variables|Default|GetImpactSound) _location)
          (Effects|SpawnEmitteratLocation (Variables|Default|GetImpactEffect) _location (Math|Rotator|MakeRotfromZ _impactnormal)))))
    (:then_1
      (bind _returnvalue_2 (Effects|SpawnEmitterAttached (Variables|Default|GetPSMuzzleFlash) (Variables|Default|GetSK_TP_Weapon) (Variables|Default|GetMuzzleSocketName)))
      (Class|PrimitiveComponent|SetOwnerNoSee _returnvalue_2 true))))