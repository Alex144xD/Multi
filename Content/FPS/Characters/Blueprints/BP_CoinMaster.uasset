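; BP_CoinMaster is a team score pickup coin for multiplayer FPS, with color and value set by a selected coin type.
; On authority, character overlap adds the value to that team's score through GS_MP_FPS, then destroys the coin.
; The construction script and type OnRep both set material color and value, but disagree on Green's value.
; A visibility OnRep toggles mesh and collision, while hide and timed respawn logic is unconnected.
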(event Custom|MC_OABO
  (params (Character :type BP%20Character%20Master%20Object%20Reference))
  (Collision|SetCollisionEnabled (Variables|Default|GetSphere) "NoCollision"))

(event Custom|Server_OABO
  (params (Character :type BP%20Character%20Master%20Object%20Reference))
  (Default|AddScore (Variables|Default|GetGSRef) (Variables|/Game/FPS/Characters/Blueprints/BP_Character_Master.BP_Character_Master_C|GetTeam Character) (Variables|Default|GetCoinValue))
  (Actor|DestroyActor))

(event EventBeginPlay
  (bind _asgs_mp_fps (Utilities|Casting|CastToGS_MP_FPS (Game|GetGameState)))
  (Variables|Default|SetGSRef _asgs_mp_fps))

(event EventTick
  (params (DeltaSeconds :type Float%20%28single-precision%29)))

(event Collision|EventActorBeginOverlap
  (params (OtherActor :type Actor%20Object%20Reference))
  (Networking|SwitchHasAuthority
    (:Authority
      (bind _asbp_character_master (Utilities|Casting|CastToBP_Character_Master OtherActor))
      (CallFunction|ServerOABO _asbp_character_master))))

(fn ConstructionScript
  (bind _eselectedcoin (Variables|Default|GetESelectedCoin))
  (bind _returnvalue (Rendering|Material|CreateDynamicMaterialInstance (Variables|Default|GetSM_Coin) 0 "/Game/FPS/Materials/M_DefaultColor2.M_DefaultColor2" :!class /Script/Engine.PrimitiveComponent))
  (Variables|Default|SetDinaMatCoin _returnvalue)
  (Rendering|Material|SetVectorParameterValue (Variables|Default|GetDinaMatCoin) "Color" (Utilities|Select :Index _eselectedcoin :NewEnumerator0 "(R=1.000000,G=1.000000,B=1.000000,A=1.000000)" :NewEnumerator1 "(R=0.019199,G=1.000000,B=0.000000,A=1.000000)" :NewEnumerator2 "(R=0.000000,G=0.079818,B=1.000000,A=1.000000)" :NewEnumerator3 "(R=0.204993,G=0.000000,B=1.000000,A=1.000000)" :NewEnumerator4 "(R=1.000000,G=0.138097,B=0.000000,A=1.000000)") :!class /Script/Engine.MaterialInstanceDynamic)
  (Variables|Default|SetCoinValue (Utilities|Select :Index _eselectedcoin :NewEnumerator0 1 :NewEnumerator1 5 :NewEnumerator2 10 :NewEnumerator3 25 :NewEnumerator4 100)))

(fn OnRepIsVisible?
  (bind _sm_coin (Variables|Default|GetSM_Coin))
  (bind _sphere (Variables|Default|GetSphere))
  (if (Variables|Default|GetIsVisible?)
    (Rendering|SetVisibility _sm_coin true false)
    (Collision|SetCollisionEnabled _sphere "QueryOnly")
    (else
      (Rendering|SetVisibility _sm_coin false false)
      (Collision|SetCollisionEnabled _sphere "NoCollision"))))

(fn OnRepESelectedCoin
  (bind _eselectedcoin (Variables|Default|GetESelectedCoin))
  (Rendering|Material|SetVectorParameterValue (Variables|Default|GetDinaMatCoin) "Color" (Utilities|Select :Index _eselectedcoin :NewEnumerator0 "(R=1.000000,G=1.000000,B=1.000000,A=1.000000)" :NewEnumerator1 "(R=0.019199,G=1.000000,B=0.000000,A=1.000000)" :NewEnumerator2 "(R=0.000000,G=0.079818,B=1.000000,A=1.000000)" :NewEnumerator3 "(R=0.204993,G=0.000000,B=1.000000,A=1.000000)" :NewEnumerator4 "(R=1.000000,G=0.138097,B=0.000000,A=1.000000)") :!class /Script/Engine.MaterialInstanceDynamic)
  (Variables|Default|SetCoinValue (Utilities|Select :Index _eselectedcoin :NewEnumerator0 1 :NewEnumerator1 2 :NewEnumerator2 10 :NewEnumerator3 25 :NewEnumerator4 100)))