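; Multiplayer FPS HUD that creates the player's widgets on BeginPlay: container, team select, character station menu, and a scoreboard for FFA, CTF and TDM.
; The selected gamemode, read from the GameInstance on the server and GameState otherwise, also toggles the team choice box.
; ShowCharStationMenu opens the station menu with UI-only input.
; DrawHUD renders a full-screen scope overlay through a dynamic material driven by ScopeOpacity.
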(event Custom|ShowCharStationMenu
  (bind _returnvalue (Game|Player|GetOwningPlayerController))
  (UserInterface|Viewport|AddtoViewport (Variables|Default|GetCharStationMenu) 0)
  (Input|SetInputModeUIOnly _returnvalue (Variables|Default|GetCharStationMenu) "DoNotLock" false)
  (Variables|/Script/Engine.PlayerController|SetbShowMouseCursor _returnvalue true))

(event EventBeginPlay
  (bind _returnvalue (Game|Player|GetOwningPlayerController))
  (Utilities|FlowControl|Sequence
    (:then_0
      (bind _asgs_mp_fps (Utilities|Casting|CastToGS_MP_FPS (Game|GetGameState)))
      (Variables|Default|SetGSRef _asgs_mp_fps)
      (bind _asgi_mp_pfs (Utilities|Casting|CastToGI_MP_PFS (Game|GetGameInstance)))
      (Variables|Default|SetGIRef _asgi_mp_pfs))
    (:then_1
      (Networking|SwitchHasAuthority
        (:Authority
          (bind _returnvalue_2 (UserInterface|CreateWidget "/Game/FPS/Blueprints/BPW_Container.BPW_Container_C" _returnvalue))
          (bind _output_get (Variables|Default|SetW_ContainerRef _returnvalue_2))
          (UserInterface|Viewport|AddtoViewport _output_get 0))))
    (:then_2
      (switch Utilities|FlowControl|Switch|SwitchonEGamemodes (select (Networking|IsServer) (Variables|/Game/FPS/Blueprints/GI_MP_PFS.GI_MP_PFS_C|GetESelectedGamemode (Variables|Default|GetGIRef)) (Variables|/Game/FPS/Blueprints/GS_MP_FPS.GS_MP_FPS_C|GetESelectedGamemode (Variables|Default|GetGSRef)))
        (:NewEnumerator1
          _)
        (:NewEnumerator2
          _)
        (:NewEnumerator3
          _))
      (Networking|SwitchHasAuthority
        (:Authority
          (bind _returnvalue_3 (UserInterface|CreateWidget "/Game/FPS/Widget/UI/BPW_Scoreboard.BPW_Scoreboard_C"))
          (bind _output_get_2 (Variables|Default|SetScoreboard _returnvalue_3))
          (UserInterface|Viewport|AddtoViewport _output_get_2 0))))
    (:then_3
      (Networking|SwitchHasAuthority
        (:Authority
          (bind _returnvalue_4 (UserInterface|CreateWidget "/Game/FPS/Widget/UI/BPW_TeamSelect.BPW_TeamSelect_C" _returnvalue))
          (bind _output_get_3 (Variables|Default|SetW_TeamSelect _returnvalue_4))
          (UserInterface|Viewport|AddtoViewport _output_get_3 0)
          (Input|SetInputModeUIOnly _returnvalue _output_get_3 "DoNotLock" false)
          (Variables|/Script/Engine.PlayerController|SetbShowMouseCursor _returnvalue true))))
    (:then_4
      (switch Utilities|FlowControl|Switch|SwitchonEGamemodes (select (Networking|IsServer) (Variables|/Game/FPS/Blueprints/GI_MP_PFS.GI_MP_PFS_C|GetESelectedGamemode (Variables|Default|GetGIRef)) (Variables|/Game/FPS/Blueprints/GS_MP_FPS.GS_MP_FPS_C|GetESelectedGamemode (Variables|Default|GetGSRef)))
        (:NewEnumerator0
          (Widget|SetVisibility (Variables|/Game/FPS/Widget/UI/BPW_TeamSelect.BPW_TeamSelect_C|GetVerticalBox_TEAM (Variables|Default|GetW_TeamSelect)) "Hidden" :!label _label))
        (:NewEnumerator1
          (goto _label))
        (:NewEnumerator2
          (Widget|SetVisibility (Variables|/Game/FPS/Widget/UI/BPW_TeamSelect.BPW_TeamSelect_C|GetVerticalBox_TEAM (Variables|Default|GetW_TeamSelect)) "Visible" :!label _label_2))
        (:NewEnumerator3
          (goto _label_2))
        (:NewEnumerator4
          (goto _label))))
    (:then_5
      (bind _returnvalue_5 (Rendering|Material|CreateDynamicMaterialInstance "/Game/FPS/Materials/M_Scope.M_Scope" "None" "None" :!class /Script/Engine.KismetMaterialLibrary))
      (Variables|Default|SetScopeMaterialRef _returnvalue_5))
    (:then_6
      (bind _returnvalue_6 (UserInterface|CreateWidget "/Game/FPS/Widget/UI/BPW_CharacterStation.BPW_CharacterStation_C" (Game|Player|GetOwningPlayerController)))
      (Variables|Default|SetCharStationMenu _returnvalue_6))))

(event EventDrawHUD
  (params (SizeX :type Integer) (SizeY :type Integer))
  (bind _scopematerialref (Variables|Default|GetScopeMaterialRef))
  (Utilities|IsValid _scopematerialref
    (:Is%20Valid
      (Rendering|Material|SetScalarParameterValue _scopematerialref "scopeOpacity" (Variables|Default|GetScopeOpacity) :!class /Script/Engine.MaterialInstanceDynamic)
      (Canvas|DrawMaterial _scopematerialref 0.0 0.0 (Math|Conversions|ToFloat(Integer) SizeX) (Math|Conversions|ToFloat(Integer) SizeY) 0.0 0.0 1.0 1.0))))

(fn ConstructionScript)