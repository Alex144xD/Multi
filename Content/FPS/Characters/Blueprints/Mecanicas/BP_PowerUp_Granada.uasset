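; Grenade power-up pickup that, on overlap with a BP_Character_Master, enables grenade throwing and sets that character's grenade count to two.
; The pickup then calls its Multicas_Hiden event, which hides the mesh, disables the sphere's collision and starts a timer.
; When the timer fires, TimerItem restores visibility and query collision and flags the item as collectable again, so it respawns in place without being destroyed.
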(event Custom|Multicas_Hiden
  (Rendering|SetVisibility (Variables|Default|GetStaticMesh) false false)
  (Collision|SetCollisionEnabled (Variables|Default|GetSphere) "NoCollision")
  (Utilities|Time|SetTimerbyFunctionName 0 "TimerItem" (Variables|Default|Gettime)))

(event EventBeginPlay)

(event Collision|EventActorBeginOverlap
  (params (OtherActor :type Actor%20Object%20Reference))
  (bind _asbp_character_master (Utilities|Casting|CastToBP_Character_Master OtherActor))
  (Variables|/Game/FPS/Characters/Blueprints/BP_Character_Master.BP_Character_Master_C|SetHasGrenadePower? _asbp_character_master true)
  (Variables|/Game/FPS/Characters/Blueprints/BP_Character_Master.BP_Character_Master_C|SetCanThrowGrenade? _asbp_character_master true)
  (Variables|/Game/FPS/Characters/Blueprints/BP_Character_Master.BP_Character_Master_C|SetGrenadeCount _asbp_character_master 2)
  (CallFunction|MulticasHiden))

(event EventTick
  (params (DeltaSeconds :type Float%20%28single-precision%29)))

(fn ConstructionScript)

(fn TimerItem
  (Rendering|SetVisibility (Variables|Default|GetStaticMesh) true false)
  (Collision|SetCollisionEnabled (Variables|Default|GetSphere) "QueryOnly")
  (Variables|Default|SetbCanBeCollected? true))