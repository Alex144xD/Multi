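; Grenade projectile that puts a dash cooldown on characters caught in its blast.
; A mesh hit plays a sound and particle effect at the impact, then the authority sphere-overlaps character pawns within ExplosionRadius.
; When AffectInstigator is false, each found character receives DashColdown and DestroyActor is called inside the loop.
; The flag is never compared to the instigator, and the grenade persists if it is true or no character is found.
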(event OnComponentHit(StaticMesh)
  (params (HitComponent :type Primitive%20Component%20Object%20Reference) (OtherActor :type Actor%20Object%20Reference) (OtherComp :type Primitive%20Component%20Object%20Reference) (NormalImpulse :type Vector :default "0, 0, 0") (Hit :type Hit%20Result%20Structure%20%28by%20ref%29))
  (CallFunction|FX Hit)
  (Networking|SwitchHasAuthority
    (:Authority
      (bind _outactors (Collision|SphereOverlapActors (Transformation|GetActorLocation) (Variables|Default|GetExplosionRadius) (Utilities|Array|MakeArray "ObjectTypeQuery3") "/Game/FPS/Characters/Blueprints/BP_Character_Master.BP_Character_Master_C"))
      (for _array_element _outactors
        (bind _asbp_character_master (Utilities|Casting|CastToBP_Character_Master _array_element))
        (if (not (Variables|Default|GetbAffectInstigator?))
          (Default|DashColdown _asbp_character_master (Variables|Default|GetCooldownTime))
          (Actor|DestroyActor))))))

(event Custom|FX
  (params (Hit%20Result :type Hit%20Result%20Structure))
  (bind (_bblockinghit _binitialoverlap _time _distance _location _impactpoint _normal _impactnormal) (Collision|BreakHitResult Hit%20Result))
  (Audio|PlaySoundatLocation (Variables|Default|Getsonido) _impactpoint "0, 0, 0" 1.0 1.0 0.0 0 0 0 0)
  (Effects|SpawnEmitteratLocation (Variables|Default|GetEffect) _impactpoint (Math|Rotator|MakeRotfromZ _impactnormal)))

(event EventBeginPlay)

(event Collision|EventActorBeginOverlap
  (params (OtherActor :type Actor%20Object%20Reference)))

(event EventTick
  (params (DeltaSeconds :type Float%20%28single-precision%29)))

(fn ConstructionScript)