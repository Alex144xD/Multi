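; Multiplayer FPS GameMode that handles team- and class-based respawning and labels the level with mode and map.
; On authority BeginPlay, it caches GameInstance and GameState, fills two TextRenderActors, and sorts team starts into Lobby, Red and Blue arrays after a short delay.
; ServerRespawnPlayer spawns and possesses the chosen class pawn at random team starts, or in place for living players at a station.
; Server_SetGMGameInfo stores the selected mode and map.
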(event Custom|ServerRespawnPlayer
  (params (PlayerController :type Player%20Controller%20Object%20Reference) (Team :type E_Team%20Enum :default "NewEnumerator0") (Eclass :type EClass%20Enum :default "NewEnumerator0") (IsAtStation? :type Boolean) (IsDead? :type Boolean))
  (bind _returnvalue (Pawn|GetControlledPawn PlayerController))
  (bind _returnvalue_2 (Utilities|Select :Index Eclass :NewEnumerator0 "/Game/FPS/Characters/Blueprints/BPC_Assault.BPC_Assault_C" :NewEnumerator1 "/Game/FPS/Characters/Blueprints/BPC_BioTech.BPC_BioTech_C" :NewEnumerator2 "/Game/FPS/Characters/Blueprints/BPC_DreadNaught.BPC_DreadNaught_C" :NewEnumerator3 "/Game/FPS/Characters/Blueprints/BPC_Engineer.BPC_Engineer_C" :NewEnumerator4 "/Game/FPS/Characters/Blueprints/BPC_Recon.BPC_Recon_C"))
  (bind _loby (Variables|Default|GetLoby))
  (bind _red (Variables|Default|GetRed))
  (bind _blue (Variables|Default|Getblue))
  (bind _returnvalue_3 (Transformation|GetActorTransform _returnvalue))
  (bind _returnvalue_4 (Utilities|Select :Index Team :NewEnumerator0 _loby :NewEnumerator1 _red :NewEnumerator2 _blue))
  (bind _returnvalue_5 (Utilities|Array|Length _returnvalue_4))
  (bind _returnvalue_6 (- _returnvalue_5 1))
  (bind _returnvalue_7 (Math|Random|RandomIntegerinRange 0 _returnvalue_6))
  (bind _output (Utilities|Array|Get(acopy) _returnvalue_4 _returnvalue_7))
  (bind _returnvalue_8 (Transformation|GetActorTransform _output))
  (Utilities|IsValid PlayerController
    (:Is%20Valid
      (if IsDead?
        (bind _returnvalue_9 (Game|SpawnActorfromClass _returnvalue_2 (Math|Transform|MakeTransform (.location _returnvalue_8) (.rotation _returnvalue_8) "1.000000,1.000000,1.000000") "AdjustIfPossibleButAlwaysSpawn" "MultiplyWithRoot" 0 Team Eclass 0 :!label _label))
        (Utilities|IsValid _returnvalue_9
          (:Is%20Valid
            (Pawn|Possess PlayerController _returnvalue_9)))
        (elif (not IsAtStation?)
          (goto _label)
          (else
            (bind _returnvalue_10 (Game|SpawnActorfromClass _returnvalue_2 (Math|Transform|MakeTransform (.location _returnvalue_3) (.rotation _returnvalue_3) "1.000000,1.000000,1.000000") "AlwaysSpawn" "MultiplyWithRoot" 0 Team Eclass 0))
            (Utilities|IsValid _returnvalue_10
              (:Is%20Valid
                (Pawn|Possess PlayerController _returnvalue_10)))))))))

(event Custom|Server_SetGMGameInfo
  (params (NewParam :type EGamemodes%20Enum :default "NewEnumerator0") (NewParam2 :type Name))
  (Variables|Default|SetE_SelectedGameMode NewParam)
  (Variables|Default|SetSelectedMapName NewParam2))

(event EventBeginPlay
  (bind _returnvalue (Networking|IsServer))
  (Networking|SwitchHasAuthority
    (:Authority
      (Utilities|FlowControl|Sequence
        (:then_0
          (bind _asgi_mp_pfs (Utilities|Casting|CastToGI_MP_PFS (Game|GetGameInstance)))
          (Variables|Default|SetGIRef _asgi_mp_pfs)
          (bind _asgs_mp_fps (Utilities|Casting|CastToGS_MP_FPS (Game|GetGameState)))
          (Variables|Default|SetGSRef _asgs_mp_fps))
        (:then_1
          (Utilities|FlowControl|Delay 0.5)
          (bind _outactors (Actor|GetAllActorsOfClass "/Game/FPS/Blueprints/BP_TeamStartMaster.BP_TeamStartMaster_C"))
          (for _array_element _outactors
            (if (Utilities|Enum|Equal(Enum) (Variables|/Game/FPS/Blueprints/BP_TeamStartMaster.BP_TeamStartMaster_C|GetTeam _array_element) "NewEnumerator0")
              (Utilities|Array|Add (Variables|Default|GetLoby) _array_element)
              (elif (Utilities|Enum|Equal(Enum) (Variables|/Game/FPS/Blueprints/BP_TeamStartMaster.BP_TeamStartMaster_C|GetTeam _array_element) "NewEnumerator1")
                (Utilities|Array|Add (Variables|Default|GetRed) _array_element)
                (elif (Utilities|Enum|Equal(Enum) (Variables|/Game/FPS/Blueprints/BP_TeamStartMaster.BP_TeamStartMaster_C|GetTeam _array_element) "NewEnumerator2")
                  (Utilities|Array|Add (Variables|Default|Getblue) _array_element))))))
        (:then_2
          (bind _outactors_2 (Actor|GetAllActorsOfClass "/Script/Engine.TextRenderActor"))
          (Rendering|Components|TextRender|SetText (Variables|/Script/Engine.TextRenderActor|GetTextRender (Utilities|Array|Get(acopy) _outactors_2)) (Utilities|Text|ToText(String) (Utilities|String|EnumtoString (select _returnvalue (Variables|/Game/FPS/Blueprints/GI_MP_PFS.GI_MP_PFS_C|GetESelectedGamemode (Variables|Default|GetGIRef)) (Variables|/Game/FPS/Blueprints/GS_MP_FPS.GS_MP_FPS_C|GetESelectedGamemode (Variables|Default|GetGSRef))))))
          (Rendering|Components|TextRender|SetText (Variables|/Script/Engine.TextRenderActor|GetTextRender (Utilities|Array|Get(acopy) _outactors_2 1)) (Utilities|Text|ToText(Name) (select _returnvalue (Variables|/Game/FPS/Blueprints/GI_MP_PFS.GI_MP_PFS_C|GetSelectedMapName (Variables|Default|GetGIRef)) (Variables|/Game/FPS/Blueprints/GS_MP_FPS.GS_MP_FPS_C|GetSelectedMapName (Variables|Default|GetGSRef)))))
          (switch Utilities|FlowControl|Switch|SwitchonEGamemodes "NewEnumerator0"
            (:NewEnumerator0
              (Rendering|Components|TextRender|SetTextRenderColor (Variables|/Script/Engine.TextRenderActor|GetTextRender (Utilities|Array|Get(acopy) _outactors_2)) (Math|Conversions|ToColor(LinearColor) "(R=0.000000,G=1.000000,B=0.099035,A=1.000000)") :!label _label))
            (:NewEnumerator1
              (Rendering|Components|TextRender|SetTextRenderColor (Variables|/Script/Engine.TextRenderActor|GetTextRender (Utilities|Array|Get(acopy) _outactors_2)) (Math|Conversions|ToColor(LinearColor) "(R=1.000000,G=0.000000,B=0.036710,A=1.000000)") :!label _label_2))
            (:NewEnumerator2
              (goto _label_2))
            (:NewEnumerator3
              (goto _label_2))
            (:NewEnumerator4
              (goto _label))))))))

(fn ConstructionScript)