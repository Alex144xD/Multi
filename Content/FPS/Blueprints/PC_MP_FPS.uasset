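; Player controller for the multiplayer FPS that holds team, class and death state, handles respawn requests and toggles the in-game menu.
; Server-named events update that state and pass it to GM_FPS for respawning.
; Tab toggles a reused BPW_TeamSelect widget, hiding team selection by game mode, read from game instance or state references cached on authority.
; EndPlay either delegates session teardown to the game instance or destroys the session and opens MainMenu.
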(event Custom|ServerRequestRespawn
  (bind _returnvalue (Game|GetGameMode))
  (Utilities|IsValid _returnvalue
    (:Is%20Valid
      (bind _asgm_fps (Utilities|Casting|CastToGM_FPS _returnvalue))
      (Utilities|IsValid _asgm_fps
        (:Is%20Valid
          (Default|ServerRespawnPlayer _asgm_fps self (Variables|Default|GetTeam) (Variables|Default|GetEclass) (Variables|Default|GetIsAtStation?) (Variables|Default|GetIsDead?)))))))

(event Custom|ServerSetEclass
  (params (Eclass :type EClass%20Enum :default "NewEnumerator0"))
  (Variables|Default|SetEclass Eclass))

(event Custom|ClientSetPCISDEad
  (params (Is%20Dead :type Boolean))
  (Variables|Default|SetIsDead? Is%20Dead))

(event Custom|ServerSetPCISDEad
  (params (Is%20Dead :type Boolean))
  (bind _output_get (Variables|Default|SetIsDead? true))
  (CallFunction|ClientSetPCISDEad _output_get))

(event Custom|Server_SetPCTeam
  (params (Team :type E_Team%20Enum :default "NewEnumerator0"))
  (Variables|Default|SetTeam Team))

(event Custom|ShowIngameMenu
  (bind _self self)
  (bind _self_2 self)
  (Utilities|IsValid (Variables|Default|GetIGMRef)
    (:Is%20Valid
      _)
    (:Is%20Not%20Valid
      (bind _returnvalue (UserInterface|CreateWidget "/Game/FPS/Widget/UI/BPW_TeamSelect.BPW_TeamSelect_C" self))
      (Variables|Default|SetIGMRef _returnvalue)))
  (if (not (Widget|IsVisible (Variables|Default|GetIGMRef)))
    (UserInterface|Viewport|AddtoViewport (Variables|Default|GetIGMRef) 0)
    (Variables|/Game/FPS/Widget/UI/BPW_TeamSelect.BPW_TeamSelect_C|SetIsAllowedBypass? (Variables|Default|GetIGMRef) true)
    (switch Utilities|FlowControl|Switch|SwitchonEGamemodes (select (Networking|IsServer) (Variables|/Game/FPS/Blueprints/GI_MP_PFS.GI_MP_PFS_C|GetESelectedGamemode (Variables|Default|GetGIRef)) (Variables|/Game/FPS/Blueprints/GS_MP_FPS.GS_MP_FPS_C|GetESelectedGamemode (Variables|Default|GetGSRef)))
      (:NewEnumerator0
        (Widget|SetVisibility (Variables|/Game/FPS/Widget/UI/BPW_TeamSelect.BPW_TeamSelect_C|GetVerticalBox_TEAM (Variables|Default|GetIGMRef)) "Hidden" :!label _label))
      (:NewEnumerator1
        (goto _label))
      (:NewEnumerator2
        _)
      (:NewEnumerator3
        _)
      (:NewEnumerator4
        (goto _label)))
    (Widget|SetVisibility (Variables|/Game/FPS/Widget/UI/BPW_TeamSelect.BPW_TeamSelect_C|GetVerticalBox_Class (Variables|Default|GetIGMRef)) "Hidden")
    (Input|SetInputModeGameandUI _self_2 (Variables|Default|GetIGMRef) "LockAlways" true false)
    (Variables|/Script/Engine.PlayerController|SetbShowMouseCursor _self_2 true)
    (Widget|SetIsEnabled (Variables|/Game/FPS/Widget/UI/BPW_TeamSelect.BPW_TeamSelect_C|GetResume (Variables|Default|GetIGMRef)) true)
    (else
      (Input|SetInputModeGameOnly _self false)
      (Variables|/Script/Engine.PlayerController|SetbShowMouseCursor _self false)
      (Widget|RemovefromParent (Variables|Default|GetIGMRef)))))

(event Custom|ClientLeaveGame
  (|DestroySession self
    (:OnSuccess
      _)
    (:OnFailure
      _))
  (Game|OpenLevel(byName) "MainMenu"))

(event EventEndPlay
  (params (EndPlayReason :type EEndPlayReason%20Enum :default "Destroyed"))
  (switch Utilities|FlowControl|Switch|SwitchonEEndPlayReason EndPlayReason
    (:Destroyed
      (bind _asgi_mp_pfs (Utilities|Casting|CastToGI_MP_PFS (Game|GetGameInstance)))
      (Default|DestroySessionCaller _asgi_mp_pfs))
    (:RemovedFromWorld
      (CallFunction|ClientLeaveGame :!label _label))
    (:Quit
      (goto _label))))

(event EventBeginPlay
  (Networking|SwitchHasAuthority
    (:Authority
      (bind _asgi_mp_pfs (Utilities|Casting|CastToGI_MP_PFS (Game|GetGameInstance)))
      (Variables|Default|SetGIRef _asgi_mp_pfs)
      (bind _asgs_mp_fps (Utilities|Casting|CastToGS_MP_FPS (Game|GetGameState)))
      (Variables|Default|SetGSRef _asgs_mp_fps))))

(event Input|KeyboardEvents|Tab
  (params (Key :type Key%20Structure :default "None"))
  (:Pressed
    (CallFunction|ShowIngameMenu)))

(fn ConstructionScript)