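; Multiplayer FPS game state that runs the match countdown, tallies Red and Blue team scores, and stores the selected game mode and map.
; BeginPlay reads match time from GI_MP_PFS as hours if it equals 1, otherwise minutes.
; For FFA, CTF and TDM, authority starts a looping one-second timer that decrements a timespan, formats TimerText and clears itself at zero.
; AddScore adds coin values to team totals.
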(event Custom|Server_SetGameInfo
  (params (SelectedEgamemode :type EGamemodes%20Enum :default "NewEnumerator0") (SelectedMapName :type Name))
  (Variables|Default|SetESelectedGamemode SelectedEgamemode)
  (Variables|Default|SetSelectedMapName SelectedMapName))

(event Custom|CountDownTimer
  (bind _timertimespan (Variables|Default|GetTimerTimeSpan))
  (bind _hours (Variables|Default|Gethours))
  (bind _minutes (Variables|Default|GetMinutes))
  (bind _days (Variables|Default|Getdays))
  (bind _returnvalue (+ (.seconds _timertimespan) _days))
  (bind _returnvalue_2 (+ (.hours _timertimespan) _hours))
  (bind _returnvalue_3 (+ (.minutes _timertimespan) _minutes))
  (bind (_days_2 _hours_2 _minutes_2 _seconds) (Math|Timespan|BreakTimespan (Math|Timespan|MakeTimespan (.days _timertimespan) _returnvalue_2 _returnvalue_3 _returnvalue (.milliseconds _timertimespan))))
  (CallFunction|SubtractSeconds)
  (Variables|Default|SettimerText (Utilities|Text|FormatText "{H}:{M}:{S}" (Utilities|Text|ToText(Integer) _hours_2 false true 1 2) (Utilities|Text|ToText(Integer) _minutes_2 false true 2 2) (Utilities|Text|ToText(Integer) _seconds false true 2 2)))
  (if (Math|Boolean|ANDBoolean (== _hours_2 0) (== _minutes_2 0) (== _seconds 0))
    (Utilities|FlowControl|DoOnce false
      (:Completed
        (Utilities|Time|ClearandInvalidateTimerbyHandle (Variables|Default|GetCountDownTimerHandle))))))

(event Custom|AddScore
  (params (Team :type E_Team%20Enum :default "NewEnumerator0") (CoinValue :type Integer))
  (switch Utilities|FlowControl|Switch|SwitchonE_Team Team
    (:NewEnumerator1
      (Variables|Default|SetRedTeamScore (+ (Variables|Default|GetRedTeamScore) CoinValue)))
    (:NewEnumerator2
      (Variables|Default|SetBlueTeamScore (+ (Variables|Default|GetBlueTeamScore) CoinValue)))))

(event EventBeginPlay
  (bind _timertimespan (Variables|Default|GetTimerTimeSpan))
  (Utilities|FlowControl|Sequence
    (:then_0
      (bind _asgi_mp_pfs (Utilities|Casting|CastToGI_MP_PFS (Game|GetGameInstance)))
      (Variables|Default|SetGIRef _asgi_mp_pfs))
    (:then_1
      (if (== (Variables|/Game/FPS/Blueprints/GI_MP_PFS.GI_MP_PFS_C|GetMatchTime (Variables|Default|GetGIRef)) 1)
        (Variables|Default|Sethours (Variables|/Game/FPS/Blueprints/GI_MP_PFS.GI_MP_PFS_C|GetMatchTime (Variables|Default|GetGIRef)))
        (else
          (Variables|Default|SetMinutes (Variables|/Game/FPS/Blueprints/GI_MP_PFS.GI_MP_PFS_C|GetMatchTime (Variables|Default|GetGIRef))))))
    (:then_2
      (switch Utilities|FlowControl|Switch|SwitchonEGamemodes (Variables|/Game/FPS/Blueprints/GI_MP_PFS.GI_MP_PFS_C|GetESelectedGamemode (Variables|Default|GetGIRef))
        (:NewEnumerator1
          _)
        (:NewEnumerator2
          _)
        (:NewEnumerator3
          _))
      (Networking|SwitchHasAuthority
        (:Authority
          (Variables|Default|SettimerText (Utilities|Text|FormatText "{H}:{M}:{S}" (Utilities|Text|ToText(Integer) (.Hours (Math|Timespan|BreakTimespan (Math|Timespan|MakeTimespan (.days _timertimespan) (+ (.hours _timertimespan) (Variables|Default|Gethours)) (+ (.minutes _timertimespan) (Variables|Default|GetMinutes)) (+ (.seconds _timertimespan) (Variables|Default|Getdays)) (.milliseconds _timertimespan)))) false true 1 2) (Utilities|Text|ToText(Integer) (.Minutes (Math|Timespan|BreakTimespan (Math|Timespan|MakeTimespan (.days _timertimespan) (+ (.hours _timertimespan) (Variables|Default|Gethours)) (+ (.minutes _timertimespan) (Variables|Default|GetMinutes)) (+ (.seconds _timertimespan) (Variables|Default|Getdays)) (.milliseconds _timertimespan)))) false true 2 2) (Utilities|Text|ToText(Integer) (.Seconds (Math|Timespan|BreakTimespan (Math|Timespan|MakeTimespan (.days _timertimespan) (+ (.hours _timertimespan) (Variables|Default|Gethours)) (+ (.minutes _timertimespan) (Variables|Default|GetMinutes)) (+ (.seconds _timertimespan) (Variables|Default|Getdays)) (.milliseconds _timertimespan)))) false true 2 2)))
          (bind _returnvalue (Utilities|Time|SetTimerbyEvent (delegate Custom|CountDownTimer) 1.0 true))
          (Variables|Default|SetCountDownTimerHandle _returnvalue))))))

(fn ConstructionScript)

(fn SubtractSeconds
  (bind _secondstimespan (Variables|Default|GetSecondsTimeSpan))
  (Variables|Default|SetTimerTimeSpan (- (Variables|Default|GetTimerTimeSpan) (Math|Timespan|MakeTimespan (.days _secondstimespan) (.hours _secondstimespan) (.minutes _secondstimespan) (+ (.seconds _secondstimespan) 1) (.milliseconds _secondstimespan)))))