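; BP_CoinSpawnerMaster is a server-side spawner that scatters random-type coins over the landscape while fewer than ten exist.
; A looping one-second timer sphere-traces from a random point in SpawnerVolume, sized by the construction script.
; The trace end multiplies a second random point by a negative Z vector, landing at world X/Y zero rather than directly below.
; Only Landscape hits spawn a BP_CoinMaster, slightly above impact, skipped if collision cannot be resolved.
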(event Custom|SphereTrace
  (bind _ecointype (Variables|Default|GetECoinType))
  (bind _spawnervolume (Variables|Default|GetSpawnerVolume))
  (bind _returnvalue (Transformation|GetWorldLocation _spawnervolume))
  (bind _returnvalue_2 (Components|Box|GetScaledBoxExtent _spawnervolume))
  (bind _returnvalue_3 (Math|Random|RandomPointinBoundingBox _returnvalue _returnvalue_2))
  (bind _outactors (Actor|GetAllActorsOfClass "/Game/FPS/Characters/Blueprints/BP_CoinMaster.BP_CoinMaster_C"))
  (if (< (Utilities|Array|Length _outactors) 10)
    (Variables|Default|SetESelectedCoin (Utilities|Array|Get(acopy) _ecointype (Math|Random|RandomIntegerinRange 0 (- (Utilities|Array|Length _ecointype) 1))))
    (bind (_outhit _returnvalue_4) (Collision|SphereTraceByChannel _returnvalue_3 (* _returnvalue_3 "0, 0,-1000.000000") 1e+02 "TraceTypeQuery1" false (Utilities|Array|MakeArray self) "ForDuration"))
    (if _returnvalue_4
      (Utilities|Casting|CastToBP_CoinMaster (.HitActor (Collision|BreakHitResult _outhit))
        (:CastFailed
          (Utilities|Casting|CastToBP_Character_Master (.HitActor (Collision|BreakHitResult _outhit))
            (:CastFailed
              (Utilities|Casting|CastToLandscape (.HitActor (Collision|BreakHitResult _outhit)))
              (Game|SpawnActorfromClass "/Game/FPS/Characters/Blueprints/BP_CoinMaster.BP_CoinMaster_C" (Math|Transform|MakeTransform (+ (.ImpactPoint (Collision|BreakHitResult _outhit)) "0, 0,75.000000") "0, 0, 0" "1,1,1") "AdjustIfPossibleButDontSpawnIfColliding" 0 (Variables|Default|GetESelectedCoin) 0))))))))

(event EventBeginPlay
  (Networking|SwitchHasAuthority
    (:Authority
      (Utilities|Time|SetTimerbyEvent (delegate Custom|SphereTrace) 1.0 true))))

(event Collision|EventActorBeginOverlap
  (params (OtherActor :type Actor%20Object%20Reference)))

(event EventTick
  (params (DeltaSeconds :type Float%20%28single-precision%29)))

(fn ConstructionScript
  (Components|Box|SetBoxExtent (Variables|Default|GetSpawnerVolume) (Variables|Default|GetBoxExtent) true))