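; Game instance for a multiplayer FPS that manages menu flow, single-player start and LAN session hosting, joining and teardown.
; Menu events create widgets for main, multiplayer, server list, host settings and team-select in-game menu toggle.
; Hosting opens the chosen map as a listen server.
; Single-player and hosted starts share a two-second delayed handoff of gamemode and map to the game state and game mode.
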(event Custom|StartSession
  (params (SelectedGamemode :type EGamemodes%20Enum :default "NewEnumerator0") (MapName :type Name) (MaxPlayers :type Integer) (MatchTime :type Integer))
  (bind _returnvalue (Game|GetPlayerController 0))
  (Variables|Default|SetESelectedGamemode SelectedGamemode)
  (Variables|Default|SetSelectedMapName MapName)
  (Variables|Default|SetMaxPlayersInt MaxPlayers)
  (Variables|Default|SetMatchTime MatchTime)
  (|Session _returnvalue (Variables|Default|GetMaxPlayersInt) true true
    (:OnSuccess
      (Game|OpenLevel(byName) (Variables|Default|GetSelectedMapName) true "listen")
      (Input|SetInputModeGameOnly _returnvalue false)
      (Variables|/Script/Engine.PlayerController|SetbShowMouseCursor _returnvalue false)
      (Utilities|FlowControl|Delay 2.0)
      (bind _asgs_mp_fps (Utilities|Casting|CastToGS_MP_FPS (Game|GetGameState)))
      (bind _output_get (Variables|Default|SetGSRef _asgs_mp_fps))
      (Default|ServerSetGameInfo _output_get (Variables|Default|GetESelectedGamemode) (Variables|Default|GetSelectedMapName))
      (bind _asgm_fps (Utilities|Casting|CastToGM_FPS (Game|GetGameMode)))
      (Default|ServerSetGMGameInfo _asgm_fps (Variables|Default|GetESelectedGamemode) (Variables|Default|GetSelectedMapName)))
    (:OnFailure
      (Development|PrintString "Host Game Failed" true true "(R=1.000000,G=0.007958,B=0.000000,A=1.000000)"))))

(event Custom|ShowServerList
  (bind _returnvalue (UserInterface|CreateWidget "/Game/FPS/Widget/UI/BPW_ServerList.BPW_ServerList_C" (Game|GetPlayerController 0)))
  (Variables|Default|SetServerListRef _returnvalue)
  (UserInterface|Viewport|AddtoViewport (Variables|Default|GetServerListRef) 0))

(event Custom|DestroySessionCaller
  (params (PlayerController :type Player%20Controller%20Object%20Reference))
  (bind _serversettingsref (Variables|Default|GetServerSettingsRef))
  (bind _combobox_gamemodes (Variables|/Game/FPS/Widget/BPW_ServerSettings.BPW_ServerSettings_C|GetComboBox_Gamemodes _serversettingsref))
  (Utilities|IsValid _serversettingsref
    (:Is%20Valid
      (Class|ComboBoxString|ClearOptions _combobox_gamemodes)
      (Class|ComboBoxString|ClearSelection _combobox_gamemodes))
    (:Is%20Not%20Valid
      _))
  (Variables|Default|SetESelectedGamemode "NewEnumerator0")
  (Variables|Default|SetSelectedMapName "None")
  (Variables|Default|SetMaxPlayersInt 0)
  (Variables|Default|SetMatchTime 0)
  (|DestroySession PlayerController))

(event Custom|ShowMultimplayerMenu
  (bind _returnvalue (UserInterface|CreateWidget "/Game/FPS/Widget/UI/BPW_MultiplayerMenu.BPW_MultiplayerMenu_C" (Game|GetPlayerController 0)))
  (Variables|Default|SetMultiMenuRef _returnvalue)
  (UserInterface|Viewport|AddtoViewport (Variables|Default|GetMultiMenuRef) 0))

(event Custom|ShowIngameMenu
  (bind _returnvalue (Game|GetPlayerController 0))
  (bind _returnvalue_2 (Game|GetPlayerController 0))
  (Utilities|IsValid (Variables|Default|GetIGMRef)
    (:Is%20Valid
      _)
    (:Is%20Not%20Valid
      (bind _returnvalue_3 (UserInterface|CreateWidget "/Game/FPS/Widget/UI/BPW_TeamSelect.BPW_TeamSelect_C" (Game|GetPlayerController 0)))
      (Variables|Default|SetIGMRef _returnvalue_3)))
  (if (not (Widget|IsVisible (Variables|Default|GetIGMRef)))
    (UserInterface|Viewport|AddtoViewport (Variables|Default|GetIGMRef) 0)
    (Variables|/Game/FPS/Widget/UI/BPW_TeamSelect.BPW_TeamSelect_C|SetIsAllowedBypass? (Variables|Default|GetIGMRef) true)
    (Widget|SetVisibility (Variables|/Game/FPS/Widget/UI/BPW_TeamSelect.BPW_TeamSelect_C|GetVerticalBox_Class (Variables|Default|GetIGMRef)) "Hidden")
    (Input|SetInputModeGameandUI _returnvalue_2 (Variables|Default|GetIGMRef) "LockAlways" true false)
    (Variables|/Script/Engine.PlayerController|SetbShowMouseCursor _returnvalue_2 true)
    (Widget|SetIsEnabled (Variables|/Game/FPS/Widget/UI/BPW_TeamSelect.BPW_TeamSelect_C|GetResume (Variables|Default|GetIGMRef)) true)
    (else
      (Input|SetInputModeGameOnly _returnvalue false)
      (Variables|/Script/Engine.PlayerController|SetbShowMouseCursor _returnvalue false)
      (Widget|RemovefromParent (Variables|Default|GetIGMRef)))))

(event Custom|HostGame
  (bind _returnvalue (UserInterface|CreateWidget "/Game/FPS/Widget/BPW_ServerSettings.BPW_ServerSettings_C" (Game|GetPlayerController 0)))
  (Variables|Default|SetServerSettingsRef _returnvalue)
  (UserInterface|Viewport|AddtoViewport (Variables|Default|GetServerSettingsRef) 0))

(event Custom|StartSP
  (bind _returnvalue (Game|GetPlayerController 0))
  (Variables|Default|SetSelectedMapName "Infinity")
  (Variables|Default|SetESelectedGamemode "NewEnumerator0")
  (Game|OpenLevel(byName) "Infinity")
  (Input|SetInputModeGameOnly _returnvalue false)
  (Variables|/Script/Engine.PlayerController|SetbShowMouseCursor _returnvalue false)
  (Utilities|FlowControl|Delay 2.0)
  (bind _asgs_mp_fps (Utilities|Casting|CastToGS_MP_FPS (Game|GetGameState)))
  (bind _output_get (Variables|Default|SetGSRef _asgs_mp_fps))
  (Default|ServerSetGameInfo _output_get (Variables|Default|GetESelectedGamemode) (Variables|Default|GetSelectedMapName))
  (bind _asgm_fps (Utilities|Casting|CastToGM_FPS (Game|GetGameMode)))
  (Default|ServerSetGMGameInfo _asgm_fps (Variables|Default|GetESelectedGamemode) (Variables|Default|GetSelectedMapName)))

(event Custom|JoinSesion
  (params (sesion :type Blueprint%20Session%20Result%20Structure))
  (|JoinSession (Game|GetPlayerController 0) sesion
    (:OnFailure
      (Development|PrintString "Join sesion Failed" true true "(R=1.000000,G=0.007958,B=0.000000,A=1.000000)"))))

(event Custom|ShowMainMenu
  (bind _returnvalue (Game|GetPlayerController 0))
  (bind _returnvalue_2 (UserInterface|CreateWidget "/Game/FPS/Widget/UI/BPW_MainMenu.BPW_MainMenu_C" _returnvalue))
  (Variables|Default|SetMainMenuRef _returnvalue_2)
  (UserInterface|Viewport|AddtoViewport (Variables|Default|GetMainMenuRef) 0)
  (Input|SetInputModeUIOnly _returnvalue 0 "DoNotLock" false)
  (Variables|/Script/Engine.PlayerController|SetbShowMouseCursor _returnvalue true))